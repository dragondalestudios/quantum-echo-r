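; Player-controlled Paper2D side-scrolling character that walks, runs, jumps, crouches and crawls along the X axis.
; Input actions set state flags, which the Walk axis event reads to move the character, choose walk or run speed and select the sprite flipbook.
; Tick flips facing by setting control yaw from X velocity.
; The sprite component is set to replicate, and interact input only updates grab and interact flags.
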(event EventTick
  (params (DeltaSeconds :type Float%20%28single-precision%29))
  ;[1 1 1] Tick - Updates animation
  (Math|Float|CompareFloat (.X (Math|Vector|BreakVector (Variables|/Script/Engine.MovementComponent|GetVelocity (Pawn|GetMovementComponent)))) 0.0
    (:>
      (Pawn|SetControlRotation (Pawn|GetController) (Math|Rotator|MakeRotator 0.0 0.0 0.0)))
    (:<
      (Pawn|SetControlRotation (Pawn|GetController) (Math|Rotator|MakeRotator 0.0 0.0 1.8e+02)))))

(event EventOnLanded
  (params (Hit :type Hit%20Result%20Structure%20%28by%20ref%29))
  ;[1 1 1] Handle movement (todo: alter jump values based on walk/run state)
  (Variables|Default|SetIsJumping false))

(event EventBeginPlay
  (Class|ActorComponent|SetIsReplicated (Variables|Default|GetSprite) true)
  (Variables|Default|SetEMoveMode "NewEnumerator0"))

(event Input|ActionEvents|InputActionCrawl
  (params (Key :type Key%20Structure :default "AnyKey"))
  ;[1 1 1] Handle movement (todo: alter jump values based on walk/run state)
  (:Pressed
    (Variables|Default|SetIsCrawling true)
    (Character|Crouch))
  (:Released
    (Variables|Default|SetIsCrawling false)
    (Character|UnCrouch)))

(event Input|ActionEvents|InputActionRun
  (params (Key :type Key%20Structure :default "AnyKey"))
  ;[1 1 1] Handle movement (todo: alter jump values based on walk/run state)
  (:Pressed
    (Variables|Default|SetIsRunning true))
  (:Released
    (Variables|Default|SetIsRunning false)))

(event Input|ActionEvents|InputActionCrouch
  (params (Key :type Key%20Structure :default "AnyKey"))
  ;[1 1 1] Handle movement (todo: alter jump values based on walk/run state)
  (:Pressed
    (Variables|Default|SetIsCrouching true)
    (Character|Crouch))
  (:Released
    (Variables|Default|SetIsCrouching false)
    (Character|UnCrouch)))

(event Input|ActionEvents|InputActioninteract
  (params (Key :type Key%20Structure :default "AnyKey"))
  ;[1 1 1] Handle movement (todo: alter jump values based on walk/run state)
  (:Pressed
    (Variables|Default|SetIsGrabbing true))
  (:Released
    (Variables|Default|SetIsGrabbing false)
    (if (Variables|Default|Getis_interacting)
      (Variables|Default|Setis_interacting false)
      (else
        (Variables|Default|Setis_interacting true)))))

(event Input|ActionEvents|InputActionJump
  (params (Key :type Key%20Structure :default "AnyKey"))
  ;[1 1 1] Handle movement (todo: alter jump values based on walk/run state)
  (:Pressed
    (Variables|Default|SetIsJumping true)
    (Character|Jump))
  (:Released
    (Variables|Default|SetIsJumping false)
    (Character|StopJumping)))

(event Input|AxisEvents|InputAxisWalk
  (params (AxisValue :type Float%20%28single-precision%29))
  ;[1 1 1] Handle movement (todo: alter jump values based on walk/run state)
  (bind _output_get (Variables|Default|SetAxisValue AxisValue))
  (bind _output_get_2 (Variables|Default|SetIsWalking (!= _output_get 0.0)))
  (if _output_get_2
    (Pawn|Input|AddMovementInput "1.000000, 0, 0" (Variables|Default|GetAxisValue) false)
    (if (Variables|Default|GetIsCrouching)
      (Sprite|SetFlipbook (Variables|Default|GetSprite) "/Game/Sprites/Character/Crouch/ANIM_Char_Crouch_WalkAlt.ANIM_Char_Crouch_WalkAlt")
      (elif (Variables|Default|GetIsCrawling)
        (Sprite|SetFlipbook (Variables|Default|GetSprite) "/Game/Sprites/Character/Crawl/ANIM_Char_CrawlMove.ANIM_Char_CrawlMove")
        (elif (Variables|Default|GetIsRunning)
          (Variables|/Script/Engine.CharacterMovementComponent|SetMaxWalkSpeed (Variables|Character|GetCharacterMovement) (Variables|Default|GetRunSpeed))
          (if (Variables|Default|GetIsJumping)
            (Sprite|SetFlipbook (Variables|Default|GetSprite) "/Game/Sprites/Character/Jump/ANIM_Char_Jump.ANIM_Char_Jump")
            (else
              (Sprite|SetFlipbook (Variables|Default|GetSprite) "/Game/Sprites/Character/Run/ANIM_Char_Run.ANIM_Char_Run")))
          (else
            (Variables|/Script/Engine.CharacterMovementComponent|SetMaxWalkSpeed (Variables|Character|GetCharacterMovement) (Variables|Default|GetWalkSpeed))
            (if (Variables|Default|GetIsJumping)
              (Sprite|SetFlipbook (Variables|Default|GetSprite) "/Game/Sprites/Character/Jump/ANIM_Char_Jump.ANIM_Char_Jump")
              (else
                (Sprite|SetFlipbook (Variables|Default|GetSprite) "/Game/Sprites/Character/Walk/ANIM_Char_Walk.ANIM_Char_Walk")))))))
    (elif (Variables|Default|GetIsCrouching)
      (Sprite|SetFlipbook (Variables|Default|GetSprite) "/Game/Sprites/Character/Crouch/ANIM_Char_Crouch.ANIM_Char_Crouch")
      (elif (Variables|Default|GetIsCrawling)
        (Sprite|SetFlipbook (Variables|Default|GetSprite) "/Game/Sprites/Character/Crawl/ANIM_Char_Crawl.ANIM_Char_Crawl")
        (elif (Variables|Default|GetIsJumping)
          (Sprite|SetFlipbook (Variables|Default|GetSprite) "/Game/Sprites/Character/Jump/ANIM_Char_Jump.ANIM_Char_Jump")
          (else
            (Sprite|SetFlipbook (Variables|Default|GetSprite) "/Game/Sprites/Character/Idle/ANIM_Char_Idle.ANIM_Char_Idle")))))))

(fn ConstructionScript)