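; A grabbable 2D sprite object that the player character (BP_QE_Character) can carry.
; Every Tick it checks whether the cached player is grabbing and overlapping its Box.
; While held, it turns red, moves to a carry position and is constrained to the character's sprite with swing locked.
; Otherwise it turns white, breaks the constraint and frees swing, though CalculateCarryPosition contains only an unconnected vector node.
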(event EventBeginPlay
  (CallFunction|SetupCharacter))

(event EventTick
  (params (DeltaSeconds :type Float%20%28single-precision%29))
  (bind _physicsconstraint (Variables|Default|GetPhysicsConstraint))
  (bind _physicsconstraint_2 (Variables|Default|GetPhysicsConstraint))
  (bind _grabbing (CallFunction|CheckCharacterGrab))
  (if _grabbing
    (Sprite|SetSpriteColor (Variables|Default|GetPaperSprite) "(R=1.000000,G=0.000000,B=0.000000,A=1.000000)")
    (Transformation|SetWorldLocation (Variables|Default|GetPaperSprite) (Utilities|CalculateCarryPosition) false false)
    (Class|PhysicsConstraintComponent|SetConstrainedComponents (Variables|Default|GetPhysicsConstraint) (Variables|Default|GetPaperSprite) "None" (Variables|/Script/Paper2D.PaperCharacter|GetSprite (Variables|Default|GetCharacter)) "None")
    (Class|PhysicsConstraintComponent|SetAngularSwing1Limit _physicsconstraint_2 "ACM_Locked" 0.0)
    (Class|PhysicsConstraintComponent|SetAngularSwing2Limit _physicsconstraint_2 "ACM_Locked" 0.0)
    (else
      (Sprite|SetSpriteColor (Variables|Default|GetPaperSprite) "(R=1.000000,G=1.000000,B=1.000000,A=1.000000)")
      (Class|PhysicsConstraintComponent|BreakConstraint (Variables|Default|GetPhysicsConstraint))
      (Class|PhysicsConstraintComponent|SetAngularSwing1Limit _physicsconstraint "ACM_Free" 0.0)
      (Class|PhysicsConstraintComponent|SetAngularSwing2Limit _physicsconstraint "ACM_Free" 0.0))))

(fn ConstructionScript)

(fn SetupCharacter
  (bind _asbp_qe_character (Utilities|Casting|CastToBP_QE_Character (Game|GetPlayerCharacter 0)))
  (Variables|Default|SetCharacter _asbp_qe_character))

(fn CheckCharacterGrab
  (bind _output_get (Variables|Default|SetPlayerGrabbing (and (Variables|/Game/Blueprints/Game/BP_QE_Character.BP_QE_Character_C|GetIsGrabbing (Variables|Default|GetCharacter)) (Collision|IsOverlappingActor (Variables|Default|GetBox) (Variables|Default|GetCharacter) :!class /Script/Engine.PrimitiveComponent))))
  (return _output_get))